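; Player controller for the vehicle game that handles pawn spawning, HUD setup, scoreboard registration and powerup use.
; On BeginPlay in VehicleAdvExampleMap, authority spawns and possesses a vehicle, picking PlayerStart location and rotation by separate random rolls.
; Initialization creates powerup and minimap widgets and registers a file-loaded name with BP_ScoreManager.
; LeftCtrl consumes the current powerup; only the mine has an effect, while the others just print.
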(event Custom|CheckFlagCollision
  (params (CollisionWith :type Vehicle%20Animation%20Blueprint%20Object%20Reference)))

(event Custom|RegisterAtScoreManager
  ;[1 1 1] Register at ScoreManager
  (bind _outactors (Actor|GetAllActorsOfClass "/Game/VehicleAdvBP/Blueprints/BP_ScoreManager.BP_ScoreManager_C"))
  (bind _result (Class|FileIO|LoadStringfromFile "Test"))
  (Development|PrintString _result)
  (bind _output_get (Variables|Default|SetScoreboardName _result))
  (Default|AddPlayerEvent (Utilities|Array|Get(acopy) _outactors) _output_get))

(event Custom|SetCurrentPowerup
  (params (PowerupIndex :type Integer))
  ;[1 1 1] Set Current Powerup
  (Variables|Default|SetCurrentPowerup PowerupIndex)
  (Default|UpdatePowerupImage (Variables|Default|GetPowerupWidget) (Variables|Default|GetCurrentPowerup)))

(event Custom|AddPawn
  (Networking|SwitchHasAuthority
    (:Authority
      (bind _outactors (Actor|GetAllActorsOfClass "/Script/Engine.PlayerStart"))
      ;[1 1 1] Add Pawn
      (bind _returnvalue (Game|SpawnActorfromClass "/Game/VehicleAdvBP/Blueprints/VehicleBlueprint.VehicleBlueprint_C" (Math|Transform|MakeTransform (Transformation|GetActorLocation (Utilities|Array|Get(acopy) _outactors (Math|Random|RandomIntegerinRange 0 (- (Utilities|Array|Length _outactors) 1)))) (Transformation|GetActorRotation (Utilities|Array|Get(acopy) _outactors (Math|Random|RandomIntegerinRange 0 (- (Utilities|Array|Length _outactors) 1))))) "AlwaysSpawn" 0 0))
      (Development|PrintString "Adding vehiclebp" true true "(R=0.000000,G=0.660000,B=1.000000,A=1.000000)" 1e+02)
      (Pawn|Possess _returnvalue))))

(event Custom|ActivatePowerup
  (params (Powerup :type Integer))
  ;[1 1 1] Activate Powerup
  (switch int Powerup
    (:1
      (Development|PrintString "Activating powerup 1"))
    (:2
      (Development|PrintString "Activating powerup 2"))
    (:3
      (Development|PrintString "Activating powerup 3")
      (CallFunction|SpawnMine))))

(event Custom|Initialize
  ;[1 1 1] Initialize
  (CallFunction|InitializePowerupWidget)
  (CallFunction|RegisteratScoreManager)
  (bind _returnvalue (UserInterface|CreateWidget "/Game/VehicleAdvBP/Blueprints/BP_Minimap.BP_Minimap_C"))
  (UserInterface|Viewport|AddtoViewport _returnvalue 0))

(event EventBeginPlay
  ;[1 1 1] BeginPlay
  (bind _returnvalue (Game|GetCurrentLevelName true))
  (if (Utilities|Enum|Equal(Enum) _returnvalue "VehicleAdvExampleMap")
    (CallFunction|AddPawn)
    (CallFunction|Initialize)))

(event Input|KeyboardEvents|LeftCtrl
  (params (Key :type Key%20Structure :default "AnyKey"))
  ;[1 1 1] LeftCtrl Pressed
  (:Pressed
    (CallFunction|ActivatePowerup (Variables|Default|GetCurrentPowerup))
    (CallFunction|SetCurrentPowerup)))

(fn ConstructionScript)

(fn SpawnMine
  (Game|SpawnActorfromClass "/Game/VehicleAdvBP/Blueprints/BP_Mine.BP_Mine_C" (Math|Transform|MakeTransform (Transformation|GetActorLocation (Pawn|GetControlledPawn))) "AlwaysSpawn" 0 0))

(fn InitializePowerupWidget
  (bind _returnvalue (UserInterface|CreateWidget "/Game/VehicleAdvBP/Blueprints/W_Powerup.W_Powerup_C"))
  (UserInterface|Viewport|AddtoViewport _returnvalue 0)
  (Variables|Default|SetPowerupWidget _returnvalue)
  (CallFunction|SetCurrentPowerup))

(fn InitializeMinimapWidget
  (bind _returnvalue (UserInterface|CreateWidget "/Game/VehicleAdvBP/Blueprints/BP_Minimap.BP_Minimap_C" (Game|GetPlayerController 0)))
  (UserInterface|Viewport|AddtoViewport _returnvalue 0))