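; Game mode for the vehicle game that provides events to host, join and quit multiplayer games.
; Hosting clears all widgets, creates a four-connection online session and opens VehicleAdvExampleMap as a listen server.
; Joining uses the passed-in session result.
; BeginPlay, EndPlay and RespawnPlayer are empty; disconnected leftover nodes cover session teardown, vehicle spawn and possession, and score manager lookup.
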(event Custom|Respawn%20Player
  (params (Player%20Controller :type BP%20Player%20Controller%20Object%20Reference))
  ;[1 1 1] Respawn Player
)

(event Custom|QuitGame
  (Game|QuitGame (Game|GetPlayerController 0) "Quit"))

(event Custom|HostGame
  ;[1 1 1] Host Game
  (Viewport|RemoveAllWidgets)
  (|Session (Game|GetPlayerController 0) 4 false
    (:OnSuccess
      (Game|OpenLevel(byName) "VehicleAdvExampleMap" true "listen"))))

(event Custom|JoinGame
  (params (Session :type Blueprint%20Session%20Result%20Structure))
  ;[1 1 1] Join Game
  (|JoinSession (Game|GetPlayerController 0) Session))

(event EventBeginPlay
  ;[1 1 1] BeginPlay
)

(event EventTick
  (params (DeltaSeconds :type Float%20%28single-precision%29)))

(event EventEndPlay
  (params (EndPlayReason :type EEndPlayReason%20Enum :default "Destroyed"))
  ;[1 1 1] EndPlay
)

(fn ConstructionScript)