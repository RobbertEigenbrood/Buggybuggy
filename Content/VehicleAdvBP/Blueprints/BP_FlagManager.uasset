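; Flag manager for a capture-the-flag mode that keeps a flag in play and awards points for captures.
; On BeginPlay it spawns a BP_Flag at the Cube location of a random entry in FlagSpawnPoints.
; FlagCaptured credits the flag owner's scoreboard name through the first BP_ScoreManager found in the world, then destroys the flag and spawns a replacement at another random pick.
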(event Custom|Flag%20Captured
  (bind _flag (Variables|Default|GetFlag))
  (bind _score_manager (CallFunction|GetScoreManager))
  (bind _playercontroller (Default|GetOwningPlayerController _flag))
  (Default|AddScoretoPlayerNameEvent _score_manager (Variables|/Game/VehicleAdvBP/Blueprints/BP_PlayerController.BP_PlayerController_C|GetScoreboardName _playercontroller) (Variables|Default|GetFlagCaptureScore))
  (Actor|DestroyActor _flag)
  (CallFunction|SpawnFlagatRandomPoint))

(event Custom|SpawnFlagAtRandomPoint
  (bind _location (CallFunction|GetRandomFlagSpawnPoint 0.0))
  (bind _returnvalue (Game|SpawnActorfromClass "/Game/VehicleAdvBP/Blueprints/BP_Flag.BP_Flag_C" _location "AlwaysSpawn" 0 0))
  (Variables|Default|SetFlag _returnvalue))

(event EventBeginPlay
  (CallFunction|SpawnFlagatRandomPoint))

(fn ConstructionScript)

(fn GetRandomFlagSpawnPoint
  (params (ZOffset :type Float%20%28single-precision%29))
  (bind _flagspawnpoints (Variables|Default|GetFlagSpawnPoints))
  (return (Math|Transform|MakeTransform (+ (Math|Vector|MakeVector 0.0 0.0 ZOffset) (Transformation|GetWorldLocation (Variables|/Game/VehicleAdvBP/Blueprints/BP_FlagSpawnPoint.BP_FlagSpawnPoint_C|GetCube (Utilities|Array|Get(acopy) _flagspawnpoints (Math|Random|RandomIntegerinRange 0 (- (Utilities|Array|Length _flagspawnpoints) 1)))))))))

(fn GetGameMode
  (bind _asbp_game_mode (Utilities|Casting|CastToBP_GameMode (Game|GetGameMode))
    (:then
      (return _asbp_game_mode))
    (:CastFailed
      (Development|PrintString "BP_FlagManager: No GameMode found"))))

(fn GetScoreManager
  (bind _outactors (Actor|GetAllActorsOfClass "/Game/VehicleAdvBP/Blueprints/BP_ScoreManager.BP_ScoreManager_C"))
  (return (Utilities|Array|Get(acopy) _outactors)))