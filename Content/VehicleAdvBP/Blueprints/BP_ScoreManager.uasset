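; Score manager that tracks each player's score by name and creates the W_Scoreboard widget on screen at BeginPlay.
; Events register players at zero and add points by finding the name in the PlayerScores struct array and rewriting that entry.
; Helper functions expose the array, look up single scores and generate numbered player names from the array length.
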(event Custom|AddPlayerEvent
  (params (PlayerController :type String))
  (CallFunction|AddPlayer PlayerController)
  (Development|PrintString "Adding player in scoremanager"))

(event Custom|AddScoreToPlayerNameEvent
  (params (playerName :type String) (score :type Integer))
  (CallFunction|AddScoretoPlayerName playerName score))

(event EventBeginPlay
  (bind _returnvalue (UserInterface|CreateWidget "/Game/VehicleAdvBP/Blueprints/W_Scoreboard.W_Scoreboard_C"))
  (UserInterface|Viewport|AddtoViewport _returnvalue 0)
  (Variables|Default|SetScoreboard _returnvalue))

(fn ConstructionScript)

(fn AddScoretoPlayerName
  (params (Player :type String) (Score :type Integer))
  (bind _playerscores (Variables|Default|GetPlayerScores))
  (bind _playerscore (CallFunction|GetIndexOfPlayerName Player))
  (Utilities|Array|SetArrayElem _playerscores _playerscore (Utilities|Struct|MakePlayerScore (.PlayerName (Utilities|Struct|BreakPlayerScore (Utilities|Array|Get(acopy) _playerscores _playerscore))) (+ (.Score (Utilities|Struct|BreakPlayerScore (Utilities|Array|Get(acopy) _playerscores _playerscore))) Score))))

(fn GetScoreArray
  (return (Variables|Default|GetPlayerScores)))

(fn GetScoreforPlayerName
  (params (PlayerName :type String))
  (for _array_element (Variables|Default|GetPlayerScores)
    (if (Utilities|Enum|Equal(Enum) PlayerName (.PlayerName (Utilities|Struct|BreakPlayerScore _array_element)))
      (return (.Score (Utilities|Struct|BreakPlayerScore _array_element)))))
  (return (.Score (Utilities|Struct|BreakPlayerScore _array_element))))

(fn IncrementPlayerScore
  (params (Player :type String) (Score :type Integer))
  (bind _playerscores (Variables|Default|GetPlayerScores))
  (for (_array_element _array_index) _playerscores
    (if (Utilities|Enum|Equal(Enum) Player (.PlayerName (Utilities|Struct|BreakPlayerScore _array_element)))
      (Utilities|Array|SetArrayElem _playerscores _array_index (Utilities|Struct|MakePlayerScore Player (+ (.Score (Utilities|Struct|BreakPlayerScore _array_element)) Score))))))

(fn AddPlayer
  (params (Player%20name :type String))
  (Utilities|Array|Add (Variables|Default|GetPlayerScores) (Utilities|Struct|MakePlayerScore Player%20name))
  (return ""))

(fn GetIndexOfPlayerName
  (params (playerName :type String))
  (for (_array_element _array_index) (Variables|Default|GetPlayerScores)
    (if (Utilities|Enum|Equal(Enum) (.PlayerName (Utilities|Struct|BreakPlayerScore _array_element)) playerName)
      (return _array_index)))
  (Development|PrintString (Utilities|String|Append "Player score for name not found: " playerName)))

(fn CreatePlayerName
  (return (Utilities|String|Append "Player " (Utilities|String|ToString(Integer) (+ (Utilities|Array|Length (Variables|Default|GetPlayerScores)) 1)))))