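; Spawner actor that keeps a powerup of a configurable type available in the vehicle game.
; On BeginPlay it spawns the powerup at its Base component's location plus an offset, always spawning regardless of collision, and hands it a reference back to the spawner.
; The PowerupPickedUp event waits SpawnDelay seconds, then spawns a replacement.
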(event Custom|PowerupPickedUp
  (Utilities|FlowControl|Delay (Variables|Default|GetSpawnDelay))
  (CallFunction|SpawnPowerup))

(event EventBeginPlay
  (CallFunction|SpawnPowerup))

(event EventActorBeginOverlap
  (params (OtherActor :type Actor%20Object%20Reference)))

(fn ConstructionScript)

(fn SpawnPowerup
  (bind _newparam (CallFunction|GetSpawnTransform))
  (bind _returnvalue (Game|SpawnActorfromClass (Variables|Default|GetPowerupType) _newparam "AlwaysSpawn" 0 0))
  (Variables|/Game/VehicleAdvBP/Blueprints/BP_Powerup.BP_Powerup_C|SetSpawnerReference _returnvalue self))

(fn GetSpawnTransform
  (return (Math|Transform|MakeTransform (+ (Transformation|GetWorldLocation (Variables|Default|GetBase)) (Variables|Default|GetSpawnOffset)))))