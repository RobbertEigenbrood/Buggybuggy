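; BP_Gate is a gate actor in the VehicleAdvBP content that can be switched active or inactive.
; ActivateGate sets the Active flag, makes the Box query-only, shows GateArrow and registers itself as ActiveGate on the first BP_GateManager found in the level.
; DeactivateGate clears the flag, disables the Box's collision and hides the arrow, without updating the manager.
; The gate has no overlap or tick logic of its own.
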(event Custom|DeactivateGate
  (Variables|Default|SetActive false)
  (Collision|SetCollisionEnabled (Variables|Default|GetBox) "NoCollision")
  (Rendering|SetVisibility (Variables|Default|GetGateArrow) false false))

(event Custom|ActivateGate
  (Variables|Default|SetActive true)
  (Collision|SetCollisionEnabled (Variables|Default|GetBox) "QueryOnly")
  (Rendering|SetVisibility (Variables|Default|GetGateArrow) true false)
  (bind _outactors (Actor|GetAllActorsOfClass "/Game/VehicleAdvBP/Blueprints/BP_GateManager.BP_GateManager_C"))
  (Variables|/Game/VehicleAdvBP/Blueprints/BP_GateManager.BP_GateManager_C|SetActiveGate (Utilities|Array|Get(acopy) _outactors) self))

(event EventActorBeginOverlap
  (params (OtherActor :type Actor%20Object%20Reference)))

(event EventTick
  (params (DeltaSeconds :type Float%20%28single-precision%29)))

(event EventBeginPlay)

(fn ConstructionScript)