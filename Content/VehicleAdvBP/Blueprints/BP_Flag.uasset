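; BP_Flag is a capture-the-flag pickup that vehicles carry, steal from one another and deliver to a gate.
; Overlapping a vehicle snaps the flag pole to that vehicle's Arrow and starts a short delay before it can change hands again.
; Tick polls the carrier's Box for overlapping vehicles to pass the flag on.
; Overlapping a BP_Gate detaches the flag and notifies the level's BP_FlagManager of the capture.
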(event OnComponentBeginOverlap(Box)
  (params (OtherActor :type Actor%20Object%20Reference) (OtherComp :type Primitive%20Component%20Object%20Reference) (OtherBodyIndex :type Integer) (bFromSweep :type Boolean) (SweepResult :type Hit%20Result%20Structure%20%28by%20ref%29))
  (bind _asvehicle_blueprint (Utilities|Casting|CastToVehicleBlueprint OtherActor)
    (:then
      (CallFunction|AttachFlagtoVehicle _asvehicle_blueprint))
    (:CastFailed
      (Utilities|Casting|CastToBP_Gate OtherActor)
      (CallFunction|HandleGateCollision))))

(event Custom|SetCaptureDelay
  (params (Delay :type Float%20%28single-precision%29))
  (Variables|Default|SetFlagIsCapturable false)
  (Utilities|FlowControl|Delay Delay)
  (Variables|Default|SetFlagIsCapturable true))

(event Custom|DetachFlagFromCurrentParent
  (Class|SceneComponent|DetachfromParent (Variables|Default|GetFlagPole) true true))

(event Custom|HandleVehicleCollision
  (params (Vehicle :type Vehicle%20Blueprint%20Object%20Reference))
  (bind _different (CallFunction|VehicleIsDifferentfromParent Vehicle))
  (if _different
    (if (Variables|Default|GetFlagIsCapturable)
      (CallFunction|AttachFlagtoVehicle Vehicle))))

(event Custom|HandleGateCollision
  (CallFunction|DetachFlagfromCurrentParent)
  (bind _flagmanager (CallFunction|GetFlagManager))
  (Default|FlagCaptured _flagmanager))

(event Custom|AttachFlagToVehicle
  (params (Vehicle :type Vehicle%20Blueprint%20Object%20Reference))
  (if (Variables|Default|GetFlagIsCapturable)
    (bind _output_get (Variables|Default|SetParentVehicle Vehicle))
    (Class|SceneComponent|Attachto (Variables|Default|GetFlagPole) (Variables|/Game/VehicleAdvBP/Blueprints/VehicleBlueprint.VehicleBlueprint_C|GetArrow Vehicle) "None" "SnapToTarget" false)
    (CallFunction|SetCaptureDelay 5.0)
    (Variables|Default|SetBox (Variables|/Game/VehicleAdvBP/Blueprints/VehicleBlueprint.VehicleBlueprint_C|GetBox _output_get))))

(event EventTick
  (params (DeltaSeconds :type Float%20%28single-precision%29))
  (bind _parentvehicle (Variables|Default|GetParentVehicle))
  (bind _box (Variables|/Game/VehicleAdvBP/Blueprints/VehicleBlueprint.VehicleBlueprint_C|GetBox _parentvehicle))
  (bind _overlappingactors (Collision|GetOverlappingActors _box "/Game/VehicleAdvBP/Blueprints/VehicleBlueprint.VehicleBlueprint_C" :!class /Script/Engine.PrimitiveComponent))
  (if (Utilities|IsValid (Variables|Default|GetParentVehicle))
    (if (> (Utilities|Array|Length _overlappingactors) 0)
      (bind _asvehicle_blueprint (Utilities|Casting|CastToVehicleBlueprint (Utilities|Array|Get(acopy) _overlappingactors)))
      (CallFunction|AttachFlagtoVehicle _asvehicle_blueprint))))

(fn ConstructionScript)

(fn GetOwningPlayerController
  (bind _newparam (Default|GetOwningPlayerController (Variables|Default|GetParentVehicle)))
  (return _newparam))

(fn VehicleIsDifferentfromParent
  (params (OtherVehicle :type Vehicle%20Blueprint%20Object%20Reference))
  (return (!= OtherVehicle (Variables|Default|GetParentVehicle))))

(fn GetFlagManager
  (bind _outactors (Actor|GetAllActorsOfClass "/Game/VehicleAdvBP/Blueprints/BP_FlagManager.BP_FlagManager_C"))
  (return (Utilities|Array|Get(acopy) _outactors)))