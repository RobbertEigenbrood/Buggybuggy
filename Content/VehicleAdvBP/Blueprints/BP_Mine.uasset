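; BP_Mine is a mine that blasts any vehicle that drives into it.
; After an activation delay on BeginPlay it arms itself and switches its mesh to a green material.
; Once armed, an overlap with a VehicleBlueprint applies a radial force to that vehicle's mesh, centered on the vehicle, spawns an explosion emitter there and destroys the mine.
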(event Collision|EventActorBeginOverlap
  (params (OtherActor :type Actor%20Object%20Reference))
  (if (Variables|Default|GetActivated)
    (bind _asvehicle_blueprint (Utilities|Casting|CastToVehicleBlueprint OtherActor))
    (Physics|AddRadialForce (Variables|/Script/Engine.WheeledVehicle|GetMesh _asvehicle_blueprint) (Transformation|GetActorLocation _asvehicle_blueprint) 1e+03 5e+04 "RIF_Linear" true)
    (Effects|SpawnEmitteratLocation "/Game/StarterContent/Particles/P_Explosion.P_Explosion" (Transformation|GetActorLocation _asvehicle_blueprint))
    (Actor|DestroyActor)))

(event EventBeginPlay
  (Utilities|FlowControl|Delay (Variables|Default|GetActivationDelay))
  (Variables|Default|SetActivated true)
  (Rendering|Material|SetMaterial (Variables|Default|GetMine) 0 "/Game/VehicleAdvBP/Textures/GreenMaterial.GreenMaterial"))

(event EventTick
  (params (DeltaSeconds :type Float%20%28single-precision%29)))

(fn ConstructionScript)